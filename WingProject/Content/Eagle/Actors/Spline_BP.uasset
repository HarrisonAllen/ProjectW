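; Spline actor that traces the eagle's left wing along its skeleton.
; On BeginPlay and every Tick, it finds the first Eagle_Mesh_Blueprint_Wing actor and rebuilds LeftWingSpline in world space from neck, wing base and numbered wing socket positions.
; Disconnected experiments remain for a two-wing spline, wing rotations mapped from a third-person character's arm bones, and debug prints.
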(event `self.ReceiveBeginPlay`
  ;[1 1 1] Sets the spline points along the existing bones
  (bind _outactors (`GameplayStatics.GetAllActorsOfClass` "/Game/Eagle/Actors/Eagle_Mesh_Blueprint_Wing.Eagle_Mesh_Blueprint_Wing_C" :!label _label))
  (`KismetArrayLibrary.Array_Clear` (`self.SocketPositions`))
  (bind _skeletalmeshcomponent (`SkeletalMeshActor.SkeletalMeshComponent` (`KismetArrayLibrary.Array_Get` _outactors)))
  (`KismetArrayLibrary.Array_Add` (`self.SocketPositions`) (`SceneComponent.GetSocketLocation` _skeletalmeshcomponent "Neck"))
  (`KismetArrayLibrary.Array_Add` (`self.SocketPositions`) (`SceneComponent.GetSocketLocation` _skeletalmeshcomponent "LeftWingBase"))
  (for _index (range 1 16)
    (bind _output_get (set `self.WingName` (`KismetStringLibrary.BuildString_Int` "" "LeftWing" _index)))
    (`KismetArrayLibrary.Array_Add` (`self.SocketPositions`) (`SceneComponent.GetSocketLocation` _skeletalmeshcomponent (`KismetStringLibrary.Conv_StringToName` _output_get))))
  (`SplineComponent.SetSplinePoints` (`self.LeftWingSpline`) (`self.SocketPositions`) "World" true))

(event `self.ReceiveTick`
  (params (DeltaSeconds :type "Float (single-precision)"))
  ;[1 1 1] Sets the spline points along the existing bones
  (goto _label))

(fn `UserConstructionScript`)